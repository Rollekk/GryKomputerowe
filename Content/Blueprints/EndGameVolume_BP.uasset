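; EndGameVolume_BP is a trigger volume that ends the game when the player character overlaps it while out of combat.
; The overlap check passes through a DoOnce into ShowCompleteHUD, so the ending fires only once.
; ShowCompleteHUD pauses the game, silences the music class through a sound mix override, and shows the EndGame widget with its BlendIn animation.
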(event `self.ReceiveActorBeginOverlap`
  (params (OtherActor :type "Actor Object Reference"))
  (bind _asplayer_character_bp (cast `/Game/Characters/Ninja/PlayerCharacter_BP` OtherActor))
  (if (not (`PlayerCharacter.bIsInCombat` _asplayer_character_bp))
    (`/Engine/EditorBlueprintResources/StandardMacros.DoOnce` false
      (:`Completed`
        (`self.ShowCompleteHUD`)))))

(fn `ShowCompleteHUD`
  (`GameplayStatics.SetGamePaused` true)
  (`GameplayStatics.SetBaseSoundMix` "/Game/HUD/Sounds/SoundMix.SoundMix")
  (`GameplayStatics.SetSoundMixClassOverride` "/Game/HUD/Sounds/SoundMix.SoundMix" "/Game/HUD/Sounds/MusicClass.MusicClass" 0.0 1.0 0.0)
  (bind _returnvalue (`|CreateWidget` "/Game/HUD/EndGame.EndGame_C"))
  (`UserWidget.AddToViewport` _returnvalue 0)
  (`UserWidget.PlayAnimation` _returnvalue (`/Game/HUD/EndGame.BlendIn` _returnvalue) 0.0 1 "Forward" 1.0 false))

(fn `UserConstructionScript`)